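; Game mode for a Pakman game that creates the main HUD and spawns the ghosts when play begins.
; SpawnGhosts places a ghost character at every TargetPoint in the level, cycling through color, name and tolerance-radius arrays by index modulo to vary each one.
; A GameOver event shows a result message on the HUD.
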(event Custom|GameOver
  (Default|DisplayResultText (Variables|Default|GetMainHud) "Ou yeaaaaaa!!!!"))

(event EventBeginPlay
  (bind _returnvalue (UserInterface|CreateWidget "/Game/Pakman/HUD/MainHUD.MainHUD_C" (Game|GetPlayerController 0)))
  (bind _output_get (Variables|Default|SetMainHud _returnvalue))
  (UserInterface|Viewport|AddtoViewport _output_get 0)
  (CallFunction|SpawnGhosts))

(event EventTick
  (params (DeltaSeconds :type Float%20%28single-precision%29)))

(fn ConstructionScript)

(fn SpawnGhosts
  (bind _ghostcolors (Variables|Default|GetGhostColors))
  (bind _names (Variables|Default|GetNames))
  (bind _tolerances (Variables|Default|GetTolerances))
  (bind _outactors (Actor|GetAllActorsOfClass "/Script/Engine.TargetPoint"))
  (for (_array_element _array_index) _outactors
    (bind _returnvalue (Game|SpawnActorfromClass "/Game/Pakman/PakmanGhostCharacterBP.PakmanGhostCharacterBP_C" (Transformation|GetActorTransform _array_element) "AlwaysSpawn" 0 (Utilities|Array|Get(acopy) _ghostcolors (Math|Integer|%(Integer) _array_index (Utilities|Array|Length _ghostcolors))) 0))
    (Variables|/Script/Pakman.PakmanGhostCharacter|SetName _returnvalue (Utilities|Array|Get(acopy) _names (Math|Integer|%(Integer) _array_index (Utilities|Array|Length _names))))
    (Variables|/Script/Pakman.PakmanGhostCharacter|SetToleranceRadius _returnvalue (Utilities|Array|Get(acopy) _tolerances (Math|Integer|%(Integer) _array_index (Utilities|Array|Length _tolerances))))))